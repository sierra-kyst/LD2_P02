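; Water body Blueprint child that sets up an underwater post-process effect matched to its own height in the level.
; On BeginPlay it creates a dynamic instance of M_UnderWater_PostProcess_Volume and writes the actor's world Z into the WaterZLine parameter.
; It then assigns that instance as the WaterBodyComponent's underwater post-process material before calling the parent BeginPlay.
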(event EventBeginPlay
  (bind _returnvalue (Rendering|Material|CreateDynamicMaterialInstance "/Game/_Game/Materials/M_UnderWater_PostProcess_Volume.M_UnderWater_PostProcess_Volume" "None" "None" :!class /Script/Engine.KismetMaterialLibrary))
  (Rendering|Material|SetScalarParameterValue _returnvalue "WaterZLine" (.z (Transformation|GetActorLocation)) :!class /Script/Engine.MaterialInstanceDynamic)
  (Class|WaterBodyComponent|SetUnderwaterPostProcessMaterial (Variables|Default|GetWaterBodyComponent) _returnvalue)
  (|CallParentFunction))

(event Collision|EventActorBeginOverlap
  (params (OtherActor :type Actor%20Object%20Reference))
  (|CallParentFunction OtherActor) ; This node is disabled and will not be called.\nDrag off pins to build functionality.
)

(event EventTick
  (params (DeltaSeconds :type Float%20%28single-precision%29))
  (|CallParentFunction DeltaSeconds) ; This node is disabled and will not be called.\nDrag off pins to build functionality.
)

(fn ConstructionScript
  (|CallParentFunction))