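; BP_OpenableLocker is an interactable locker that opens and closes once unlocked, yielding a key the first time it opens.
; Interaction checks Unlocked, then a FlipFlop alternates between OpenLocker and CloseLocker.
; Opening and closing swap visibility between two components, MOC for open and MCC for closed, with no animation.
; A DoOnce in OpenLocker spawns a single BP_Key at the Arrow component's world transform.
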(event Custom|Open%20Locker
  (Rendering|SetVisibility (Variables|Default|GetM_C_C) false false)
  (Rendering|SetVisibility (Variables|Default|GetM_O_C) true false)
  (Utilities|FlowControl|DoOnce false
    (:Completed
      (Game|SpawnActorfromClass "/Game/_Game/Blueprints/InteractionActors/BP_Key.BP_Key_C" (Transformation|GetWorldTransform (Variables|Default|GetArrow)) "Undefined" "MultiplyWithRoot" 0 0))))

(event Custom|Close%20Locker
  (Rendering|SetVisibility (Variables|Default|GetM_O_C) false false)
  (Rendering|SetVisibility (Variables|Default|GetM_C_C) true false))

(event EventInteraction
  (if (Variables|Default|GetUnlocked?)
    (Utilities|FlowControl|FlipFlop
      (:A
        (CallFunction|OpenLocker))
      (:B
        (CallFunction|CloseLocker)))))

(fn ConstructionScript)