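; BP_Padlock is an interactable padlock that the player removes by spending a key.
; On Interaction it reads the key count from the first-person player controller and, if at least one key is held, decrements it and calls UnlockLock.
; UnlockLock plays a 2D unlock sound and destroys the padlock actor.
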(event Custom|UnlockLock
  (Audio|PlaySound2D "/Game/_Game/Audio/door_unlock_Cue.door_unlock_Cue" 1.0 1.0 0.0 0 0)
  (Actor|DestroyActor))

(event EventInteraction
  (bind _asbp_first_person_player_controller (Utilities|Casting|CastToBP_FirstPersonPlayerController (Game|GetPlayerController 0)))
  (if (>= (Variables|/Game/FirstPerson/Blueprints/BP_FirstPersonPlayerController.BP_FirstPersonPlayerController_C|GetKeys _asbp_first_person_player_controller) 1)
    (Variables|/Game/FirstPerson/Blueprints/BP_FirstPersonPlayerController.BP_FirstPersonPlayerController_C|SetKeys _asbp_first_person_player_controller (- (Variables|/Game/FirstPerson/Blueprints/BP_FirstPersonPlayerController.BP_FirstPersonPlayerController_C|GetKeys _asbp_first_person_player_controller) 1))
    (CallFunction|UnlockLock)))

(fn ConstructionScript)