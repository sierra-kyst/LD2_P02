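; Interactable locked door that opens if the player controller holds at least one key and can later slam shut for a jumpscare.
; Interaction with a key swings it open once via timeline, then disables actor collision, without decrementing the key count.
; Without a key, a short timeline jiggles the door.
; The Jumpscare event swings it back to closed, then plays a slam sound and restores collision.
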(event Custom|Jumpscare
  ;[1 1 1] Jumpscare
  (bind _alpha (Timeline|Timeline_2 Play)
    (:Update
      (Transformation|SetRelativeRotation (Variables|Default|Getдвкрь_Куб) (Math|Rotator|MakeRotator 0.0 0.0 (Math|Float|Lerp 6e+01 -48.0 _alpha)) false false))
    (:Finished
      (Audio|PlaySoundatLocation "/Game/_Game/Audio/door_slam_Cue.door_slam_Cue" (Transformation|GetWorldLocation (Variables|Default|Getдвкрь_Куб_003)) "0, 0, 0" 1.0 1.0 0.0 0 0 0 0)
      (Collision|SetActorEnableCollision true))))

(event EventInteraction
  (bind _asbp_first_person_player_controller (Utilities|Casting|CastToBP_FirstPersonPlayerController (Game|GetPlayerController 0)))
  (if (>= (Variables|/Game/FirstPerson/Blueprints/BP_FirstPersonPlayerController.BP_FirstPersonPlayerController_C|GetKeys _asbp_first_person_player_controller) 1)
    (Utilities|FlowControl|DoOnce false
      (:Completed
        (Audio|PlaySoundatLocation "/Game/_Game/Audio/door_open_Cue.door_open_Cue" (Transformation|GetWorldLocation (Variables|Default|Getдвкрь_Куб_003)) "0, 0, 0" 1.0 1.0 0.0 0 0 0 0)
        (bind _alpha (Timeline|Timeline_0 Play)
          (:Update
            (Transformation|SetRelativeRotation (Variables|Default|Getдвкрь_Куб) (Math|Rotator|MakeRotator 0.0 0.0 (Math|Float|Lerp -48.0 6e+01 _alpha)) false false))
          (:Finished
            (Collision|SetActorEnableCollision false)))))
    (else
      (Audio|PlaySoundatLocation 0 (Transformation|GetWorldLocation (Variables|Default|Getдвкрь_Куб_003)) "0, 0, 0" 1.0 1.0 0.0 0 0 0 0) ; Struggle with locked door sound
      (bind _alpha_2 (Timeline|Timeline_1 PlayFromStart)
        (:Update
          (Transformation|SetRelativeRotation (Variables|Default|Getдвкрь_Куб) (Math|Rotator|MakeRotator 0.0 0.0 (Math|Float|Lerp -48.0 -47.0 _alpha_2)) false false))))))

(fn ConstructionScript
  (|CallParentFunction))