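; BP_Screw is an interactable screw that the player can turn and remove once the screwdriver is obtained.
; Interaction checks ScrewdriverGet on the first-person player controller, counts the turn and plays a sound.
; The ScrewTurn timeline lerps the screw's yaw and Z offset through two separate alpha tracks.
; Its update destroys the actor as soon as the turn count reaches two, without waiting for the animation to finish.
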(event EventInteraction
  (bind _asbp_first_person_player_controller (Utilities|Casting|CastToBP_FirstPersonPlayerController (Game|GetPlayerController 0)))
  (if (Variables|/Game/FirstPerson/Blueprints/BP_FirstPersonPlayerController.BP_FirstPersonPlayerController_C|GetScrewdriverGet _asbp_first_person_player_controller)
    (Variables|Default|SetTurns (+ (Variables|Default|GetTurns) 1))
    (Audio|PlaySound2D 0 1.0 1.0 0.0 0 0)
    (bind (_direction _alpha _alpha2) (Timeline|Screw%20Turn Play)
      (:Update
        (Transformation|SetRelativeLocationAndRotation (Variables|Default|Getscrew) (Math|Vector|MakeVector 0.0 0.0 (Math|Float|Lerp 0.0 0.75 _alpha2)) (Math|Rotator|MakeRotator 0.0 0.0 (Math|Float|Lerp 0.0 -9e+01 _alpha)) false false)
        (if (>= (Variables|Default|GetTurns) 2)
          (Actor|DestroyActor))))))

(fn ConstructionScript)