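; BP_Dial is one rotating number dial of a combination lock, with an arrow widget that it initializes with itself.
; RotateDial plays a click sound and turns the dial mesh one tenth of a revolution on a timeline, ignoring input until the turn finishes.
; When finished, it wraps the angle at a full turn, derives and prints the current number, and tells the owning lock to check the combination.
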(event Custom|FindNumber
  (bind _output_get (Variables|Default|SetNumber (Math|Float|Truncate (/ (Variables|Default|GetDialRotation) 36.0))))
  (Development|PrintString (Utilities|String|ToString(Integer) _output_get)))

(event Custom|RotateDial
  (if (Variables|Default|GetCanRotate)
    (Variables|Default|SetCanRotate false)
    (Audio|PlaySound2D "/Game/_Game/Audio/CombinationLockClick_Cue.CombinationLockClick_Cue" 1.0 1.0 0.0 0 0)
    (bind _alpha (Timeline|DialRotation_TL PlayFromStart)
      (:Update
        (Transformation|SetRelativeRotation (Variables|Default|GetSM_Dial) (Math|Rotator|MakeRotator 0.0 0.0 (+ (Variables|Default|GetDialRotation) (Math|Float|Lerp 0.0 36.0 _alpha))) false false))
      (:Finished
        (Variables|Default|SetDialRotation (+ (Variables|Default|GetDialRotation) (Math|Float|Lerp 0.0 36.0 _alpha)))
        (if (>= (Variables|Default|GetDialRotation) 3.6e+02)
          (Variables|Default|SetDialRotation 0.0)
          (Transformation|SetRelativeRotation (Variables|Default|GetSM_Dial) "0, 0, 0" false false))
        (CallFunction|FindNumber)
        (Default|CheckEveryTurn (Variables|Default|GetLockRef))
        (Variables|Default|SetCanRotate true)))))

(event EventBeginPlay
  (bind _aswbp_arrow (Utilities|Casting|CastToWBP_Arrow (UserInterface|GetUserWidgetObject (Variables|Default|GetArrow))))
  (Default|Initialize _aswbp_arrow self))

(fn ConstructionScript)