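; BP_Vent is a vent that swings open once its referenced screws are no longer all valid.
; Tick checks four screw references and plays a timeline as soon as any one of them is invalid, rather than waiting for all four.
; The timeline alpha drives a pitch lerp on the Vents component, rotating it a quarter turn from its closed position.
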(event EventTick
  (params (DeltaSeconds :type Float%20%28single-precision%29))
  (if (!= (Math|Boolean|ANDBoolean (Utilities|IsValid (Variables|Default|GetBP_Screw)) (Utilities|IsValid (Variables|Default|GetBP_Screw1)) (Utilities|IsValid (Variables|Default|GetBP_Screw2)) (Utilities|IsValid (Variables|Default|GetBP_Screw3))) true)
    (bind _alpha (Timeline|Timeline Play)
      (:Update
        (Transformation|SetRelativeRotation (Variables|Default|Getvents) (Math|Rotator|MakeRotator 0.0 (Math|Float|Lerp 0.0 -9e+01 _alpha) 0.0) false false)))))

(fn ConstructionScript)